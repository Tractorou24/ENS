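; Spike trap that repeatedly moves its Spikes along Z, starting after an initial Lag delay.
; A timeline sets the relative height, then the cycle waits WaitingTime and loops through a Restart event.
; In parallel, DamageCollision becomes visible after DamageTime and is hidden when the timeline finishes, with only visibility toggled here.
; A Debug flag unhides a Cube in game.
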(event Custom|Restart
  (bind _spikes (Variables|Default|GetSpikes))
  (bind _relativelocation (Variables|/Script/Engine.SceneComponent|GetRelativeLocation _spikes))
  (Variables|Default|SetStartPosition (Math|Vector|MakeVector (.x _relativelocation) (.y _relativelocation) (.z _relativelocation)))
  (Utilities|FlowControl|Sequence
    (:then_0
      (bind _elevation (Timeline|Timeline PlayFromStart)
        (:Update
          (Transformation|SetRelativeLocation _spikes (Math|Vector|MakeVector (.X (Math|Vector|BreakVector (Variables|Default|GetStartPosition))) (.Y (Math|Vector|BreakVector (Variables|Default|GetStartPosition))) _elevation) false false))
        (:Finished
          (Rendering|SetVisibility (Variables|Default|GetDamageCollision) false true)
          (Utilities|FlowControl|Delay (Variables|Default|GetWaitingTime))
          (CallFunction|Restart))))
    (:then_1
      (Utilities|FlowControl|Delay (Variables|Default|GetDamageTime))
      (Rendering|SetVisibility (Variables|Default|GetDamageCollision) true true))))

(event EventBeginPlay
  (bind _spikes (Variables|Default|GetSpikes))
  (bind _relativelocation (Variables|/Script/Engine.SceneComponent|GetRelativeLocation _spikes))
  (if (Variables|Default|GetDebug)
    (Development|SetHiddeninGame (Variables|Default|GetCube) false false))
  (Utilities|FlowControl|Delay (Variables|Default|GetLag))
  (Variables|Default|SetStartPosition (Math|Vector|MakeVector (.x _relativelocation) (.y _relativelocation) (.z _relativelocation)))
  (Utilities|FlowControl|Sequence
    (:then_0
      (bind _elevation (Timeline|Timeline PlayFromStart)
        (:Update
          (Transformation|SetRelativeLocation _spikes (Math|Vector|MakeVector (.X (Math|Vector|BreakVector (Variables|Default|GetStartPosition))) (.Y (Math|Vector|BreakVector (Variables|Default|GetStartPosition))) _elevation) false false))
        (:Finished
          (Rendering|SetVisibility (Variables|Default|GetDamageCollision) false true)
          (Utilities|FlowControl|Delay (Variables|Default|GetWaitingTime))
          (CallFunction|Restart))))
    (:then_1
      (Utilities|FlowControl|Delay (Variables|Default|GetDamageTime))
      (Rendering|SetVisibility (Variables|Default|GetDamageCollision) true true))))

(fn ConstructionScript)