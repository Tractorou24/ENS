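; BP_DoorEntryArena is a double arena door that opens for the player and shuts when combat waves start.
; Trigger overlaps play or reverse a timeline that yaws both panels, with opening gated by CanBeOpened.
; It finds the BP_MultiAreaSpawner tagged MainRoomSpawner, whose new waves close the door and clear that flag.
; The spawner-finished handler would re-enable opening but is unbound on BeginPlay, and the separate LockingDoor animation is never called.
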(event Custom|DoorClosing
  (Utilities|FlowControl|Sequence
    (:then_0
      (bind _opening_ (Timeline|DoorOpening Stop)
        (:Update
          (Transformation|SetRelativeRotation (Variables|Default|GetDoor01) (Math|Rotator|MakeRotator 0.0 0.0 _opening_) false false)
          (Transformation|SetRelativeRotation (Variables|Default|GetDoor02) (Math|Rotator|MakeRotator 0.0 0.0 _opening_) false false))))
    (:then_1
      (Timeline|DoorOpening Reverse))))

(event Custom|OnMainRoomSpawnerFinished
  (Variables|Default|SetCanBeOpened true))

(event Custom|CustomEvent
  (params (WaveNumber :type Integer))
  (CallFunction|DoorClosing)
  (Variables|Default|SetCanBeOpened false))

(event Custom|OnComponentBeginOverlap_Event
  (params (OverlappedComponent :type Primitive%20Component%20Object%20Reference) (OtherActor :type Actor%20Object%20Reference) (OtherComp :type Primitive%20Component%20Object%20Reference) (OtherBodyIndex :type Integer) (bFromSweep :type Boolean) (SweepResult :type Hit%20Result%20Structure%20%28by%20ref%29))
  ;[0 0 0] TestAnim Before Interaction is Setup
  (if (== OtherActor (Game|GetPlayerCharacter 0))
    (CallFunction|OpenDoor)))

(event Custom|OnComponentEndOverlap_Event
  (params (OverlappedComponent :type Primitive%20Component%20Object%20Reference) (OtherActor :type Actor%20Object%20Reference) (OtherComp :type Primitive%20Component%20Object%20Reference) (OtherBodyIndex :type Integer))
  ;[0 0 0] TestAnim Before Interaction is Setup
  (if (== OtherActor (Game|GetPlayerCharacter 0))
    (CallFunction|DoorClosing)))

(event Custom|OpenDoor
  (if (Variables|Default|GetCanBeOpened)
    (Utilities|FlowControl|Sequence
      (:then_0
        (bind _opening_ (Timeline|DoorOpening Stop)
          (:Update
            (Transformation|SetRelativeRotation (Variables|Default|GetDoor01) (Math|Rotator|MakeRotator 0.0 0.0 _opening_) false false)
            (Transformation|SetRelativeRotation (Variables|Default|GetDoor02) (Math|Rotator|MakeRotator 0.0 0.0 _opening_) false false))))
      (:then_1
        (Timeline|DoorOpening Play)))))

(event Custom|LockingDoor
  (bind _closingdoor (Timeline|ClosingDoor Play)
    (:Update
      (Transformation|SetRelativeRotation (Variables|Default|GetDoor01) (Math|Rotator|MakeRotator 0.0 0.0 _closingdoor) false false)
      (Transformation|SetRelativeRotation (Variables|Default|GetDoor02) (Math|Rotator|MakeRotator 0.0 0.0 _closingdoor) false false))))

(event EventBeginPlay
  (bind _collisiontestanim (Variables|Default|GetCollisionTestAnim))
  ;[0 0 0] TestAnim Before Interaction is Setup
  (Collision|AssignOnComponentBeginOverlap _collisiontestanim (delegate Custom|OnComponentBeginOverlap_Event))
  (Collision|AssignOnComponentEndOverlap _collisiontestanim (delegate Custom|OnComponentEndOverlap_Event))
  (bind _outactors (Actor|GetAllActorsOfClass "/Game/BP/Spawner/BP_MultiAreaSpawner.BP_MultiAreaSpawner_C"))
  (for _array_element _outactors
    (if (Actor|ActorHasTag _array_element "MainRoomSpawner")
      (bind _output_get (Variables|Default|SetMainRoomSpawner _array_element))
      (EventDispatchers|UnbindEventfromOnSpawnerFinished _output_get (delegate Custom|OnMainRoomSpawnerFinished))
      (EventDispatchers|BindEventtoOnNewWave _output_get (delegate Custom|CustomEvent)))))

(fn ConstructionScript)