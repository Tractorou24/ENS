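; BP_CrystalTransition is a crystal actor that floats and changes its material when the player is near.
; On BeginPlay it creates a dynamic instance of M_CrystalArena for the crystal mesh and binds the box overlap events.
; Player overlap plays a timeline driving the "Transition" scalar parameter, and leaving reverses it.
; A second timeline, started on BeginPlay, animates floating by adding its vector track to the mesh's current relative location each update.
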(event Custom|OnComponentBeginOverlap_Event
  (params (OverlappedComponent :type Primitive%20Component%20Object%20Reference) (OtherActor :type Actor%20Object%20Reference) (OtherComp :type Primitive%20Component%20Object%20Reference) (OtherBodyIndex :type Integer) (bFromSweep :type Boolean) (SweepResult :type Hit%20Result%20Structure%20%28by%20ref%29))
  ;[0 0 0] TransitionAnimation
  (if (== OtherActor (Game|Player|GetPlayerPawn 0))
    (bind _transition (Timeline|CurveTransition Play)
      (:Update
        (Rendering|Material|SetScalarParameterValue (Variables|Default|GetCrystalDynamicMaterial) "Transition" _transition :!class /Script/Engine.MaterialInstanceDynamic)))))

(event Custom|OnComponentEndOverlap_Event
  (params (OverlappedComponent :type Primitive%20Component%20Object%20Reference) (OtherActor :type Actor%20Object%20Reference) (OtherComp :type Primitive%20Component%20Object%20Reference) (OtherBodyIndex :type Integer))
  ;[0 0 0] TransitionAnimation
  (if (== OtherActor (Game|Player|GetPlayerPawn 0))
    (bind _transition (Timeline|CurveTransition Reverse)
      (:Update
        (Rendering|Material|SetScalarParameterValue (Variables|Default|GetCrystalDynamicMaterial) "Transition" _transition :!class /Script/Engine.MaterialInstanceDynamic)))))

(event Custom|FloatingStart
  (bind _sm_crystallow (Variables|Default|GetSM_CrystalLOW))
  (bind _relativelocation (Variables|/Script/Engine.SceneComponent|GetRelativeLocation _sm_crystallow))
  ;[0 0 0] FloatingAnimation
  (bind _floatingtrack (Timeline|CurveFloating PlayFromStart)
    (:Update
      (Transformation|SetRelativeLocation _sm_crystallow (Math|Vector|MakeVector (+ (.x _relativelocation) (.x _floatingtrack)) (+ (.y _relativelocation) (.y _floatingtrack)) (+ (.z _relativelocation) (.z _floatingtrack))) false false))))

(event EventBeginPlay
  (bind _box (Variables|Default|GetBox))
  (bind _returnvalue (Rendering|Material|CreateDynamicMaterialInstance "/Game/Art/Materials/ComplexMaterials/M_CrystalArena.M_CrystalArena" "None" "None" :!class /Script/Engine.KismetMaterialLibrary))
  (bind _output_get (Variables|Default|SetCrystalDynamicMaterial _returnvalue))
  (Rendering|Material|SetMaterial (Variables|Default|GetSM_CrystalLOW) 0 _output_get)
  (Collision|AssignOnComponentBeginOverlap _box (delegate Custom|OnComponentBeginOverlap_Event))
  (Collision|AssignOnComponentEndOverlap _box (delegate Custom|OnComponentEndOverlap_Event))
  (CallFunction|FloatingStart))

(fn ConstructionScript)