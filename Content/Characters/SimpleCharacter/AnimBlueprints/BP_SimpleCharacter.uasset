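; BP_SimpleCharacter is a character Blueprint that handles a grounded sword base attack.
; Pressing the SwordBaseAttack input plays the attack montage on the player 0 character's mesh, unless that character is falling.
; Movement stops and is disabled as the montage starts, then returns to Walking on completion, with no handling for interruption.
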(event EventBeginPlay)

(event Collision|EventActorBeginOverlap
  (params (OtherActor :type Actor%20Object%20Reference)))

(event EventTick
  (params (DeltaSeconds :type Float%20%28single-precision%29)))

(event Input|ActionEvents|InputActionSwordBaseAttack
  (params (Key :type Key%20Structure :default "None"))
  (:Pressed
    (if (not (AI|Components|NavMovement|IsFalling (Pawn|GetMovementComponent (Game|GetPlayerCharacter 0))))
      (Animation|Montage|PlayMontage (Variables|/Script/Engine.Character|GetMesh (Game|GetPlayerCharacter 0)) "/Game/Characters/SimpleCharacter/Animations/AN_SwordBaseAttack.AN_SwordBaseAttack"
        (:then
          (Components|Movement|StopMovementImmediately (Variables|Character|GetCharacterMovement))
          (Pawn|Components|CharacterMovement|DisableMovement (Variables|/Script/Engine.Character|GetCharacterMovement (Game|GetPlayerCharacter 0))))
        (:OnCompleted
          (Pawn|Components|CharacterMovement|SetMovementMode (Variables|/Script/Engine.Character|GetCharacterMovement (Game|GetPlayerCharacter 0)) "MOVE_Walking" 0))))))

(fn ConstructionScript)