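; BP_SkullKamikaze is a skull kamikaze character that carries an explosion attack.
; On BeginPlay it copies its detection range, explosion trigger range and attack move speed into its AI Blackboard.
; It then grants itself the BPGA_SkullKamikazeExplosion gameplay ability and writes its own delay, damage and radius values onto the ability object retrieved from the spec handle.
; The death event is empty.
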(event EventBeginPlay
  (bind _abilitysystemcomponent (Variables|Default|GetAbilitySystemComponent))
  (AI|Components|Blackboard|SetValueasFloat (AI|GetBlackboard 0) (Utilities|Name|MakeLiteralName "DetectionRange") (Variables|Default|GetDetectionRange))
  (AI|Components|Blackboard|SetValueasFloat (AI|GetBlackboard 0) (Utilities|Name|MakeLiteralName "ExplosionTriggerRange") (Variables|Default|GetExplosionTriggerRange))
  (AI|Components|Blackboard|SetValueasFloat (AI|GetBlackboard 0) (Utilities|Name|MakeLiteralName "AttackMoveSpeed") (Variables|Default|GetAttackMoveSpeed))
  (bind _returnvalue (GameplayAbilities|GiveAbility _abilitysystemcomponent "/Game/Characters/SkullKamikaze/BPGA_SkullKamikazeExplosion.BPGA_SkullKamikazeExplosion_C" 0 -1))
  (bind _asbpga_skull_kamikaze_explosion (Utilities|Casting|CastToBPGA_SkullKamikazeExplosion (.ReturnValue (Ability|GameplayAbility|GetGameplayAbilityfromSpecHandle _abilitysystemcomponent _returnvalue))))
  (Variables|/Game/Characters/SkullKamikaze/BPGA_SkullKamikazeExplosion.BPGA_SkullKamikazeExplosion_C|SetExplosionDelay _asbpga_skull_kamikaze_explosion (Variables|Default|GetExplosionDelay))
  (Variables|/Game/Characters/SkullKamikaze/BPGA_SkullKamikazeExplosion.BPGA_SkullKamikazeExplosion_C|SetDamages _asbpga_skull_kamikaze_explosion (Variables|Default|GetExplosionDamages))
  (Variables|/Game/Characters/SkullKamikaze/BPGA_SkullKamikazeExplosion.BPGA_SkullKamikazeExplosion_C|SetExplosionRadius _asbpga_skull_kamikaze_explosion (Variables|Default|GetExplosionRadius)))

(event EventOnDeathBlueprint)

(fn ConstructionScript)