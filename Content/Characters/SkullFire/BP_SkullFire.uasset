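; BP_SkullFire is an AI-controlled character, apparently a ranged enemy, that attacks with a fire shot ability.
; On BeginPlay it copies its detection, attack, movement-wait and strafe tuning variables into the Blackboard.
; It then grants BPGA_SkullFireShot through the Ability System and writes the character's shot speed and damage onto that ability instance.
; The death event is an empty stub.
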(event EventBeginPlay
  (bind _abilitysystemcomponent (Variables|Default|GetAbilitySystemComponent))
  (AI|Components|Blackboard|SetValueasFloat (AI|GetBlackboard 0) (Utilities|Name|MakeLiteralName "DetectionRange") (Variables|Default|GetDetectionRange))
  (AI|Components|Blackboard|SetValueasFloat (AI|GetBlackboard 0) (Utilities|Name|MakeLiteralName "AttackRange") (Variables|Default|GetAttackRange))
  (AI|Components|Blackboard|SetValueasFloat (AI|GetBlackboard 0) (Utilities|Name|MakeLiteralName "WaitAfterMoveTime") (Variables|Default|GetWaitAfterMoveTime))
  (Class|BlackboardComponent|SetValueasInt (AI|GetBlackboard 0) (Utilities|Name|MakeLiteralName "MaxAttackBeforeMove") (Variables|Default|GetMaxAttackBeforeMove))
  (AI|Components|Blackboard|SetValueasFloat (AI|GetBlackboard 0) (Utilities|Name|MakeLiteralName "StrafeAngle") (Variables|Default|GetStrafeAngle))
  (bind _returnvalue (GameplayAbilities|GiveAbility _abilitysystemcomponent "/Game/Characters/SkullFire/BPGA_SkullFireShot.BPGA_SkullFireShot_C" 0 -1))
  (bind _asbpga_skull_fire_shot (Utilities|Casting|CastToBPGA_SkullFireShot (.ReturnValue (Ability|GameplayAbility|GetGameplayAbilityfromSpecHandle _abilitysystemcomponent _returnvalue))))
  (Variables|/Game/Characters/SkullFire/BPGA_SkullFireShot.BPGA_SkullFireShot_C|SetSpeed _asbpga_skull_fire_shot (Variables|Default|GetFire%20Shot%20Speed))
  (Variables|/Game/Characters/SkullFire/BPGA_SkullFireShot.BPGA_SkullFireShot_C|SetDamage _asbpga_skull_fire_shot (Variables|Default|GetShotDamages)))

(event Collision|EventActorBeginOverlap
  (params (OtherActor :type Actor%20Object%20Reference)))

(event EventTick
  (params (DeltaSeconds :type Float%20%28single-precision%29)))

(event EventOnDeathBlueprint)

(fn ConstructionScript)