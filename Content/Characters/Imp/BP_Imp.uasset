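; Imp enemy character with a leap attack, a base attack and a target-circling behavior.
; BeginPlay grants both GAS abilities with their damage and copies tuning values to the AI Blackboard.
; After a cancelable windup, Attack solves custom gravity to reach the target, and Tick moves the Imp along that arc until a capsule trace hits.
; Circling runs on Tick, backs off when too close, and signals its end, like jump phases, through gameplay tags.
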(event Custom|MovingAroundTarget
  (params (DeltaTime :type Float%20%28double-precision%29))
  (bind _returnvalue (Transformation|GetActorLocation))
  (bind _returnvalue_2 (Transformation|GetActorLocation))
  (bind _self self)
  (bind _self_2 self)
  (bind _movearoundtargetminimalradius (Variables|Configurable|GetMoveAroundTargetMinimalRadius))
  (bind _returnvalue_3 (AI|GetAIController _self))
  (Utilities|FlowControl|Sequence
    (:then_0
      (Utilities|FlowControl|DoOnce false :!label _label
        (:Completed
          (bind _asynctaskproxy (GameplayTasks|TaskWaitDelay _returnvalue_3 (Variables|Configurable|GetMoveAroundDuration))
            (:then
              (Variables|Default|SetMovingAroundAsyncTask _asynctaskproxy))
            (:OnFinish
              (AI|Navigation|StopMovement _returnvalue_3)
              (Ability|GameplayEffect|AddLooseGameplayTags _self (GameplayTags|MakeLiteralGameplayTagContainer "(GameplayTags=((TagName=\"Ability.ImpMoveAroundTarget.Stop\")))"))
              (goto _label Reset))))))
    (:then_1
      (bind _asactor (Utilities|Casting|CastToActor (AI|Components|Blackboard|GetValueasObject (AI|GetBlackboard 0) (Utilities|Name|MakeLiteralName "Target"))))
      (if (>= (Math|Vector|Distance(Vector) (Transformation|GetActorLocation _asactor) _returnvalue_2) _movearoundtargetminimalradius)
        (if (not (Variables|Default|GetIsRepositioning))
          (bind _result (Class|MathAI|GetNextPointonCirclebyAngle (Transformation|GetActorLocation _asactor) _returnvalue (Variables|Configurable|GetMoveAroundTargetSpeed) DeltaTime (Variables|Default|GetMoveAroundTargetClockwise)))
          (if (AI|IsValidAILocation _result)
            (Transformation|SetActorRotation (Math|Rotator|Lerp(Rotator) (Transformation|GetActorRotation) (Math|Rotator|FindLookatRotation _returnvalue _result) 1.0))
            (Transformation|SetActorLocation _result false false)
            (Rendering|Debug|DrawDebugBox _result "5.000000,5.000000,5.000000" "(R=1.000000,G=0.078394,B=0.000000,A=1.000000)" "0, 0, 0" 1.0 0.0)))
        (else
          (|DoOnceMultiInput :!label _label_2
            (:A%20Out
              (Variables|Default|SetIsRepositioning true)
              (AI|AIMoveTo self (+ _returnvalue_2 (* (* (- _movearoundtargetminimalradius (Math|Vector|Distance(Vector) (Transformation|GetActorLocation _asactor) _returnvalue_2)) 1.3) (Transformation|GetActorForwardVector) -1.0)) 0 5.0 false
                (:then
                  (Rendering|Debug|DrawDebugBox (+ _returnvalue_2 (* (* (- _movearoundtargetminimalradius (Math|Vector|Distance(Vector) (Transformation|GetActorLocation _asactor) _returnvalue_2)) 1.3) (Transformation|GetActorForwardVector) -1.0)) "5.000000,5.000000,5.000000" "(R=1.000000,G=0.078394,B=0.000000,A=1.000000)" "0, 0, 0" 1.0 0.0))
                (:OnSuccess
                  (if (Utilities|IsValid (Variables|Default|GetMovingAroundAsyncTask)) :!label _label_3
                    (GameplayTasks|EndTask (Variables|Default|GetMovingAroundAsyncTask))
                    (AI|Navigation|StopMovement (AI|GetAIController _self_2))
                    (Ability|GameplayEffect|AddLooseGameplayTags _self_2 (GameplayTags|MakeLiteralGameplayTagContainer "(GameplayTags=((TagName=\"Ability.ImpMoveAroundTarget.Stop\")))"))
                    (goto _label_2 Reset%20In)
                    (else
                      (goto _label_2 Reset%20In))))
                (:OnFail
                  (goto _label_3))))
            (:Reset%20Out
              (Variables|Default|SetIsRepositioning false)
              (goto _label Reset))))))))

(event Custom|Attack
  (bind _returnvalue (Transformation|GetActorLocation))
  (bind _asynctaskproxy (GameplayTasks|TaskWaitDelay (AI|GetAIController self) (Variables|Configurable|GetWaitPrepareJumpTime))
    (:then
      (Variables|Default|SetPreparingJumpAsyncTask _asynctaskproxy))
    (:OnFinish
      (if (Variables|/Game/Art/Anims/Diablotin/ABP/ABP_Diablotin_01.ABP_Diablotin_01_C|GetIs%20Preparing%20Jump (Variables|Default|GetABP))
        (Variables|/Game/Art/Anims/Diablotin/ABP/ABP_Diablotin_01.ABP_Diablotin_01_C|SetIs%20Preparing%20Jump (Variables|Default|GetABP) false)
        (AI|Components|Blackboard|SetValueasBool (AI|GetBlackboard 0) (Utilities|Name|MakeLiteralName "IsPreparingJump") false)
        (Variables|/Game/Art/Anims/Diablotin/ABP/ABP_Diablotin_01.ABP_Diablotin_01_C|SetIs%20Jumping (Variables|Default|GetABP) true)
        (Variables|Default|SetIsJumping true)
        (Ability|GameplayEffect|AddLooseGameplayTags self (GameplayTags|MakeLiteralGameplayTagContainer "(GameplayTags=((TagName=\"Ability.ImpJump.Jumping\")))"))
        (bind _asactor (Utilities|Casting|CastToActor (AI|Components|Blackboard|GetValueasObject (AI|GetBlackboard 0) (Utilities|Name|MakeLiteralName "Target"))))
        (Variables|Default|SetStartLocation _returnvalue)
        (bind _returnvalue_2 (Class|MathAI|GetProjectileCustomGravity (Variables|Configurable|GetJumpAngle) (Variables|Configurable|GetJumpSpeed) (Math|Vector|Distance2D(Vector) (Transformation|GetActorLocation _asactor) _returnvalue)))
        (Variables|Default|SetJumpGravity _returnvalue_2)
        (Variables|Default|SetJumpDuration (/ (* (* (Variables|Configurable|GetJumpSpeed) 2.0) (Math|Trig|Sin(Degrees) (Variables|Configurable|GetJumpAngle))) (Variables|Default|GetJumpGravity)))
        (bind _output_get (Variables|Default|SetStartRotationYaw (.yaw (Transformation|GetActorRotation))))
        (Variables|Default|SetLastFlyControlDelta _output_get)
        (Physics|SetEnableGravity (Variables|Default|GetCapsuleComponent) false)
        (AI|Navigation|StopMovement (Pawn|GetController))))))

(event EventBeginPlay
  (bind _returnvalue (AI|GetBlackboard 0))
  (bind _abilitysystemcomponent (Variables|Default|GetAbilitySystemComponent))
  (bind _returnvalue_2 (GameplayAbilities|GiveAbility _abilitysystemcomponent "/Game/Characters/Imp/BPGA_ImpJump.BPGA_ImpJump_C" 0 -1))
  (bind _asbpga_imp_jump (Utilities|Casting|CastToBPGA_ImpJump (.ReturnValue (Ability|GameplayAbility|GetGameplayAbilityfromSpecHandle _abilitysystemcomponent _returnvalue_2))))
  (Variables|/Game/Characters/Imp/BPGA_ImpJump.BPGA_ImpJump_C|SetDamages _asbpga_imp_jump (Variables|Configurable|GetAttackDamage))
  (bind _returnvalue_3 (GameplayAbilities|GiveAbility _abilitysystemcomponent "/Game/Characters/Imp/BPGA_ImpBaseAttack.BPGA_ImpBaseAttack_C" 0 -1))
  (bind _asbpga_imp_base_attack (Utilities|Casting|CastToBPGA_ImpBaseAttack (.ReturnValue (Ability|GameplayAbility|GetGameplayAbilityfromSpecHandle _abilitysystemcomponent _returnvalue_3))))
  (Variables|/Game/Characters/Imp/BPGA_ImpBaseAttack.BPGA_ImpBaseAttack_C|SetDamages _asbpga_imp_base_attack (Variables|Configurable|GetAttackSecondaryDamage))
  (Variables|/Script/Engine.CharacterMovementComponent|SetMaxWalkSpeed (Variables|Character|GetCharacterMovement) (Variables|Configurable|GetMoveSpeed))
  (AI|Components|Blackboard|SetValueasFloat _returnvalue (Utilities|Name|MakeLiteralName "DetectionRange") (Variables|Configurable|GetDetectionRange))
  (AI|Components|Blackboard|SetValueasFloat _returnvalue (Utilities|Name|MakeLiteralName "AttackRange") (Variables|Configurable|GetAttackRange))
  (AI|Components|Blackboard|SetValueasFloat _returnvalue (Utilities|Name|MakeLiteralName "AttackSecondaryRange") (Variables|Configurable|GetAttackSecondaryRange))
  (AI|Components|Blackboard|SetValueasFloat _returnvalue (Utilities|Name|MakeLiteralName "WaitAfterMoveTime") (Variables|Configurable|GetWaitAfterMoveTime))
  (AI|Components|Blackboard|SetValueasFloat _returnvalue (Utilities|Name|MakeLiteralName "MaxAttackRange") (Variables|Configurable|GetMaxAttackRange))
  (AI|Components|Blackboard|SetValueasFloat _returnvalue (Utilities|Name|MakeLiteralName "AttackDelay") (Variables|Configurable|GetAttackDelay))
  (Class|BlackboardComponent|SetValueasInt _returnvalue (Utilities|Name|MakeLiteralName "MaxAttacking") (Variables|Configurable|GetMaxAttacking)))

(event EventTick
  (params (DeltaSeconds :type Float%20%28single-precision%29))
  (if (Variables|Default|GetIsJumping)
    (CallFunction|Jumping DeltaSeconds)
    (elif (Variables|Default|GetIsMovingAroundTarget)
      (CallFunction|MovingAroundTarget DeltaSeconds))))

(fn ConstructionScript)

(fn PrepareJump
  (Variables|/Game/Art/Anims/Diablotin/ABP/ABP_Diablotin_01.ABP_Diablotin_01_C|SetIs%20Preparing%20Jump (Variables|Default|GetABP) true)
  (AI|Components|Blackboard|SetValueasBool (AI|GetBlackboard 0) (Utilities|Name|MakeLiteralName "IsPreparingJump") true))

(fn CancelJump
  (bind _preparingjumpasynctask (Variables|Default|GetPreparingJumpAsyncTask))
  (Variables|/Game/Art/Anims/Diablotin/ABP/ABP_Diablotin_01.ABP_Diablotin_01_C|SetIs%20Preparing%20Jump (Variables|Default|GetABP) false)
  (Ability|GameplayEffect|AddLooseGameplayTags self (GameplayTags|MakeLiteralGameplayTagContainer "(GameplayTags=((TagName=\"Ability.ImpJump.Canceled\")))"))
  (AI|Components|Blackboard|SetValueasBool (AI|GetBlackboard 0) (Utilities|Name|MakeLiteralName "IsPreparingJump") false)
  (if (Utilities|IsValid _preparingjumpasynctask)
    (GameplayTasks|EndTask _preparingjumpasynctask)))

(fn GetJumpPositionbyTime
  (params (JumpTime :type Float%20%28double-precision%29))
  (bind _yaw (CallFunction|GetYaw))
  (Variables|Default|SetLastFlyControlDelta _yaw)
  (return (Math|Vector|MakeVector (* (Variables|Configurable|GetJumpSpeed) (Math|Trig|Cos(Degrees) (Variables|Configurable|GetJumpAngle)) (Math|Trig|Cos(Degrees) _yaw) JumpTime) (* (Variables|Configurable|GetJumpSpeed) (Math|Trig|Cos(Degrees) (Variables|Configurable|GetJumpAngle)) (Math|Trig|Sin(Degrees) _yaw) JumpTime) (- (* (Variables|Configurable|GetJumpSpeed) (Math|Trig|Sin(Degrees) (Variables|Configurable|GetJumpAngle)) JumpTime) (* (* (Variables|Default|GetJumpGravity) 0.5) (Math|Float|Square JumpTime))))))

(fn GetYaw
  (bind _returnvalue (Transformation|GetActorRotation))
  (bind _lastflycontroldelta (Variables|Default|GetLastFlyControlDelta))
  (bind _lastflycontroldelta_2 (Variables|Default|GetLastFlyControlDelta))
  (bind _lastflycontroldelta_3 (Variables|Default|GetLastFlyControlDelta))
  (bind _flycontrolratio (Variables|Configurable|GetFlyControlRatio))
  (bind _startrotationyaw (Variables|Default|GetStartRotationYaw))
  (bind _startrotationyaw_2 (Variables|Default|GetStartRotationYaw))
  (bind _flycontrolratio_2 (Variables|Configurable|GetFlyControlRatio))
  (bind _flycontrolratio_3 (Variables|Configurable|GetFlyControlRatio))
  (bind _startrotationyaw_3 (Variables|Default|GetStartRotationYaw))
  (bind _startrotationyaw_4 (Variables|Default|GetStartRotationYaw))
  (bind _returnvalue_2 (Math|Float|Absolute(Float) _lastflycontroldelta))
  (bind _returnvalue_3 (Math|Float|Absolute(Float) _lastflycontroldelta_2))
  (bind _returnvalue_4 (Math|Float|Absolute(Float) _lastflycontroldelta_3))
  (bind _returnvalue_5 (- (.yaw _returnvalue) _startrotationyaw_3))
  (bind _returnvalue_6 (- _returnvalue_5 3.6e+02))
  (bind _returnvalue_7 (+ _returnvalue_2 0.7))
  (bind _returnvalue_8 (- _returnvalue_2 0.7))
  (bind _returnvalue_9 (+ _returnvalue_3 0.7))
  (bind _returnvalue_10 (- _returnvalue_3 0.7))
  (bind _returnvalue_11 (+ _returnvalue_5 3.6e+02))
  (bind _returnvalue_12 (+ _returnvalue_4 0.7))
  (bind _returnvalue_13 (- _returnvalue_4 0.7))
  (bind _returnvalue_14 (* _returnvalue_5 _flycontrolratio_2))
  (bind _returnvalue_15 (* _returnvalue_6 _flycontrolratio))
  (bind _returnvalue_16 (* _returnvalue_11 _flycontrolratio_3))
  (bind _returnvalue_17 (+ _returnvalue_14 _startrotationyaw_4))
  (bind _returnvalue_18 (Math|Float|Absolute(Float) _returnvalue_17))
  (bind _returnvalue_19 (+ _returnvalue_15 _startrotationyaw))
  (bind _returnvalue_20 (+ _returnvalue_16 _startrotationyaw_2))
  (bind _returnvalue_21 (Math|Float|Absolute(Float) _returnvalue_19))
  (bind _returnvalue_22 (Math|Float|Absolute(Float) _returnvalue_20))
  (bind _returnvalue_23 (Math|Float|Clamp(Float) _returnvalue_18 _returnvalue_8 _returnvalue_7))
  (bind _returnvalue_24 (Math|Float|Clamp(Float) _returnvalue_21 _returnvalue_10 _returnvalue_9))
  (bind _returnvalue_25 (Math|Float|Clamp(Float) _returnvalue_22 _returnvalue_13 _returnvalue_12))
  (if (> _returnvalue_5 1.8e+02)
    (if (< _returnvalue_19 0.0)
      (return (* _returnvalue_24 -1.0))
      (else
        (return _returnvalue_24)))
    (elif (< _returnvalue_5 -1.8e+02)
      (if (< _returnvalue_20 0.0)
        (return (* _returnvalue_25 -1.0))
        (else
          (return _returnvalue_25)))
      (elif (< _returnvalue_17 0.0)
        (return (* _returnvalue_23 -1.0))
        (else
          (return _returnvalue_23))))))

(fn StartMovingAroundTarget
  (Variables|Default|SetIsMovingAroundTarget true)
  (Variables|Default|SetMoveAroundTargetClockwise (== (Math|Random|RandomInteger 2) 0)))

(fn StopMovingAroundTarget
  (Variables|Default|SetIsMovingAroundTarget false))

(fn Jumping
  (params (DeltaTime :type Float%20%28double-precision%29))
  (bind _output_get (Variables|Default|SetJumpTimeAccumulator (+ DeltaTime (Variables|Default|GetJumpTimeAccumulator))))
  (bind _result (Class|MathAI|GetProjectilePositionbyTime _output_get (Variables|Configurable|GetJumpAngle) (Variables|Default|GetStartRotationYaw) (Variables|Configurable|GetJumpSpeed) (Variables|Default|GetJumpGravity)))
  (bind _returnvalue (Collision|CapsuleTraceByChannel (Transformation|GetActorLocation) (+ _result (Variables|Default|GetStartLocation)) 35.0 5e+01 "TraceTypeQuery1" false 0 "ForDuration" true "(R=1.000000,G=0.000000,B=0.000000,A=1.000000)" "(R=0.000000,G=1.000000,B=0.000000,A=1.000000)" 1.0))
  (if _returnvalue
    (Variables|Default|SetIsJumping false)
    (Physics|SetEnableGravity (Variables|Default|GetCapsuleComponent) true)
    (Variables|Default|SetJumpTimeAccumulator 0.0)
    (Ability|GameplayEffect|AddLooseGameplayTags self (GameplayTags|MakeLiteralGameplayTagContainer "(GameplayTags=((TagName=\"Ability.ImpJump.Landing\")))"))
    (else
      (Transformation|SetActorLocation (+ _result (Variables|Default|GetStartLocation)) false false)))
  (if (<= (- (Variables|Default|GetJumpDuration) 0.15) (Variables|Default|GetJumpTimeAccumulator))
    (Variables|/Game/Art/Anims/Diablotin/ABP/ABP_Diablotin_01.ABP_Diablotin_01_C|SetIs%20Jumping (Variables|Default|GetABP) false)))