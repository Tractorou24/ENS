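; BP_ImpAIComponent is an AI component that spreads a sighted target among nearby Imps.
; Initialize stores the Blackboard, AI Perception and alert radius, records the owner's location as SpawnPoint, and binds perception updates.
; When sight perceives an actor, a sphere overlap finds BP_Imps within the radius and writes the first seen actor to each one's Target key.
; Target clearing exists but is unconnected, so this component never clears it.
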(event Custom|Initialize
  (params (Blackboard :type Blackboard%20Component%20Object%20Reference) (AIPerception :type AI%20Perception%20Component%20Object%20Reference) (AllyAlertRadius :type Float%20%28double-precision%29))
  (Variables|Default|SetBlackboard Blackboard)
  (Variables|Default|SetAIPerception AIPerception)
  (Variables|Default|SetAllyAlertRadius AllyAlertRadius)
  (AI|Components|Blackboard|SetValueasVector (Variables|Default|GetBlackboard) (Utilities|Name|MakeLiteralName "SpawnPoint") (Transformation|GetActorLocation (Components|GetOwner)))
  (EventDispatchers|BindEventtoOnPerceptionUpdated (Variables|Default|GetAIPerception) (delegate Custom|OnPerceptionUpdated)))

(event Custom|OnPerceptionUpdated
  (params (UpdatedActors :type Array%20of%20Actor%20Object%20References))
  (bind _aiperception (Variables|Default|GetAIPerception))
  (bind _outactors (Class|AIPerceptionComponent|GetCurrentlyPerceivedActors _aiperception "/Script/AIModule.AISense_Sight"))
  (bind _output (Utilities|Array|Get(acopy) _outactors))
  (if (Utilities|IsValid _output)
    (bind _outactors_2 (Collision|SphereOverlapActors (Transformation|GetActorLocation (Components|GetOwner)) (Variables|Default|GetAllyAlertRadius) (Utilities|Array|MakeArray "ObjectTypeQuery3") "/Game/Characters/Imp/BP_Imp.BP_Imp_C"))
    (for _array_element _outactors_2
      (AI|Components|Blackboard|SetValueasObject (AI|GetBlackboard _array_element) (Utilities|Name|MakeLiteralName "Target") _output))))

(event EventBeginPlay)

(event EventTick
  (params (DeltaSeconds :type Float%20%28single-precision%29)))