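; Base hitbox actor for the Imp that damages player characters overlapping its box colliders during a roughly quarter-second lifetime.
; It must be initialized with a damage amount and source ability, and asserts this each tick.
; Tick polls every box for overlaps, tracking hit characters so each is damaged once.
; Damage uses a GAS effect spec from the ability's avatar, with set-by-caller magnitude, applied to the target.
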(event EventBeginPlay
  (Variables|Default|SetColliders (Actor|GetComponentsByClass "/Script/Engine.BoxComponent"))
  (Utilities|FlowControl|Delay 0.25)
  (Actor|DestroyActor))

(event Collision|EventActorBeginOverlap
  (params (OtherActor :type Actor%20Object%20Reference)))

(event EventTick
  (params (DeltaSeconds :type Float%20%28single-precision%29))
  (Class|EnsBlueprintAssert|BlueprintAssert self (Variables|Default|GetIsInitialized))
  (for _array_element (Variables|Default|GetColliders)
    (for _array_element_2 (Collision|GetOverlappingActors _array_element "/Script/ENS.EnsPlayerCharacter" :!class /Script/Engine.PrimitiveComponent)
      (bind _asens_character_base (Utilities|Casting|CastToEnsCharacterBase _array_element_2)
        (:then
          (if (not (Utilities|Set|Contains (Variables|Default|GetHits) _asens_character_base))
            (CallFunction|GiveDamage _asens_character_base (Variables|Default|GetDamage))
            (Utilities|Set|Add (Variables|Default|GetHits) _asens_character_base)))
        (:CastFailed
          (Class|EnsBlueprintAssert|BlueprintAssert self false))))))

(fn ConstructionScript
  (|CallParentFunction))

(fn Initialize
  (params (Damage :type Float%20%28double-precision%29) (Ability :type Ens%20Gameplay%20Ability%20Base%20Object%20Reference))
  (Variables|Default|SetDamage Damage)
  (Variables|Default|SetAbility Ability)
  (Variables|Default|SetIsInitialized true))

(fn GiveDamage
  (params (Target :type Ens%20Character%20Base%20Object%20Reference) (Damage :type Float%20%28double-precision%29))
  (bind _ability (Variables|Default|GetAbility))
  (bind _returnvalue (Ability|GetAvatarActorfromActorInfo _ability))
  (bind _returnvalue_2 (Ability|GetAbilitySystemComponent _returnvalue))
  (bind _returnvalue_3 (Ability|GameplayEffect|AssignTagSetbyCallerMagnitude (GameplayEffects|MakeOutgoingSpec _returnvalue_2 "/Game/Characters/Player/Abilities/DevelopperTests/BPGE_Damage.BPGE_Damage_C" 0.0 (GameplayEffects|MakeEffectContext _returnvalue_2)) "(TagName=\"Ability.Damage\")" Damage))
  (GameplayEffects|ApplyGameplayEffectSpecToSelf (Ability|GetAbilitySystemComponent Target) _returnvalue_3)
  (return))