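; Player controller that tracks the player's lives, shows them in a HUD widget and handles restarting the game.
; On BeginPlay it sets Lives from LivesStart, then creates the WB_PlayerInfo widget and adds it to the viewport.
; The LostLife event only pushes the current Lives to the widget, without decrementing it.
; The Restart event reopens the L_main level by name.
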(event EventBeginPlay
  (Variables|Default|SetLives (Variables|Default|GetLivesStart))
  (bind _returnvalue (UserInterface|CreateWidget "/Game/Widget/WB_PlayerInfo.WB_PlayerInfo_C"))
  (bind _output_get (Variables|Default|SetWidget _returnvalue))
  (UserInterface|Viewport|AddtoViewport _output_get 0)
  (Default|UpdateLives _output_get (Variables|Default|GetLives)))

(event EventTick
  (params (DeltaSeconds :type Float%20%28single-precision%29)))

(event EventLostLife
  (Default|UpdateLives (Variables|Default|GetWidget) (Variables|Default|GetLives)))

(event EventRestart
  (Game|OpenLevel(byName) "L_main"))

(fn ConstructionScript)