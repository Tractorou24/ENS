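; BP_BaseHitbox is a base player attack hitbox that records the enemies overlapping its box colliders.
; It caches all its Box components on BeginPlay, then every Tick adds overlapping EnsEnemyBase actors to a Hits set, so each enemy appears only once.
; GetOverlappedEnemiesLastFrame copies and clears that set, returning an array of enemies gathered since the previous call, despite its single-frame name.
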(event EventBeginPlay
  (Variables|Default|SetColliders (Actor|GetComponentsByClass "/Script/Engine.BoxComponent")))

(event EventTick
  (params (DeltaSeconds :type Float%20%28single-precision%29))
  (for _array_element (Variables|Default|GetColliders)
    (bind _filteredarray (Utilities|Array|FilterArray (Collision|GetOverlappingActors _array_element "/Script/ENS.EnsEnemyBase" :!class /Script/Engine.PrimitiveComponent) "/Script/ENS.EnsEnemyBase"))
    (Utilities|Set|AddItems (Variables|Default|GetHits) _filteredarray)))

(fn ConstructionScript)

(fn GetOverlappedEnemiesLastFrame
  (bind _hits (Variables|Default|GetHits))
  (bind _output_get (LocalVariables|SetRetuenedHits _hits))
  (Utilities|Set|Clear _hits)
  (bind _result (Utilities|Set|ToArray _output_get))
  (return _result))