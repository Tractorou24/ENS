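; BP_Wall2MAngle_SB_01 is an art Blueprint for an angled wall piece that varies its stone blocks procedurally.
; The Construction Script randomly shows or hides six stone components by a visibility weight and stretches each on Y within a minimum-to-maximum scale range.
; Both rolls use the Seed stream, which is reseeded with a random integer on each construction run, so the layout changes whenever the script reruns.
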(event EventBeginPlay)

(event Collision|EventActorBeginOverlap
  (params (OtherActor :type Actor%20Object%20Reference)))

(event EventTick
  (params (DeltaSeconds :type Float%20%28single-precision%29)))

(fn ConstructionScript
  (bind _seed (Variables|Default|GetSeed))
  (bind _output_get (Variables|Default|SetStoneBlocks (Utilities|Array|MakeArray (Variables|Default|GetStone_07) (Variables|Default|GetStone_06) (Variables|Default|GetStone_05) (Variables|Default|GetStone_04) (Variables|Default|GetStone_03) (Variables|Default|GetStone_02))))
  (Math|Random|SetRandomStreamSeed (Variables|Default|GetSeed) (Math|Random|RandomInteger 9999))
  (for _array_element _output_get
    (Rendering|SetVisibility _array_element (Class|KismetMathLibrary|RandomBoolwithWeightfromStream _seed (Variables|Default|GetPercentageOfStoneVisible)) false)
    (Transformation|SetRelativeScale3D _array_element (Math|Vector|MakeVector 1.0 (Math|Random|RandomFloatinRangefromStream _seed (Variables|Default|GetMinimumScale) (Variables|Default|GetMaximumScale)) 1.0))))