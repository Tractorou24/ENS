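; BP_Wall2MAngle_SB_01 is an art-tool Blueprint that assembles a randomized wall piece from three mesh components: under wall, ground volume and upper wall.
; The Construction Script optionally re-rolls the Seed stream when Randomize is set, then calls Setup.
; Setup picks each mesh from its data array using the seeded stream, randomly scales the under wall and ground volume within set ranges, and can mirror the ground volume through negative Y scale.
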(event EventBeginPlay)

(event Collision|EventActorBeginOverlap
  (params (OtherActor :type Actor%20Object%20Reference)))

(event EventTick
  (params (DeltaSeconds :type Float%20%28single-precision%29)))

(fn ConstructionScript
  (if (Variables|Default|GetRandomize)
    (Math|Random|SetRandomStreamSeed (Variables|Default|GetSeed) (Math|Random|RandomInteger 9999)))
  (CallFunction|Setup))

(fn Setup
  (bind _undwall50_01 (Variables|Default|GetUndWall50_01))
  (bind _minimumscale_groundvolume (Variables|Default|GetMinimumScale_GroundVolume))
  (bind _maximumscale_groundvolume (Variables|Default|GetMaximumScale_GroundVolume))
  (bind _seed (Variables|Default|GetSeed))
  (bind _groundvolume_01 (Variables|Default|GetGroundVolume_01))
  (bind _returnvalue (Math|Random|RandomFloatinRangefromStream _seed _minimumscale_groundvolume _maximumscale_groundvolume))
  (bind _relativescale3d (Variables|/Script/Engine.SceneComponent|GetRelativeScale3D _groundvolume_01))
  (Utilities|FlowControl|Sequence
    (:then_0
      (Components|StaticMesh|SetStaticMesh _undwall50_01 (Utilities|Array|Get(acopy) (Variables|Default|GetUndWall50_Data) (Math|Random|RandomIntegerinRangefromStream (Variables|Default|GetSeed) 0 (- (Utilities|Array|Length (Variables|Default|GetUndWall50_Data)) 1))))
      (Transformation|SetRelativeScale3D _undwall50_01 (Math|Vector|MakeVector 1.0 (Math|Random|RandomFloatinRangefromStream (Variables|Default|GetSeed) (Variables|Default|GetMinimumScale_UndWall) (Variables|Default|GetMaximumScale_UndWall)) 1.0)))
    (:then_1
      (Components|StaticMesh|SetStaticMesh _groundvolume_01 (Utilities|Array|Get(acopy) (Variables|Default|GetGroundVolumes_Data) (Math|Random|RandomIntegerinRangefromStream (Variables|Default|GetSeed) 0 (- (Utilities|Array|Length (Variables|Default|GetGroundVolumes_Data)) 1))))
      (Transformation|SetRelativeScale3D _groundvolume_01 (Math|Vector|MakeVector 1.2 _returnvalue _returnvalue))
      (if (Variables|Default|GetMirrorGroundVolume)
        (Transformation|SetRelativeScale3D _groundvolume_01 (Math|Vector|MakeVector (.x _relativescale3d) (* (.y _relativescale3d) -1.0) (.z _relativescale3d)))))
    (:then_2
      (Components|StaticMesh|SetStaticMesh (Variables|Default|GetUpWall) (Utilities|Array|Get(acopy) (Variables|Default|GetUpWall_Data) (Math|Random|RandomIntegerinRangefromStream (Variables|Default|GetSeed) 0 (- (Utilities|Array|Length (Variables|Default|GetUpWall_Data)) 1)))))))