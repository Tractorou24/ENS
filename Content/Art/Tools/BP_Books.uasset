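; Editor art tool actor that procedurally builds a row of book static meshes in its construction script.
; Each book is a mesh drawn from BooksData with a seeded random stream, optionally reseeded, and placed along Y using its local bounds and a spacing value.
; Weighted rolls turn books 180 degrees with a bounds-based position correction, and coin flips add random X/Z displacement and pitch tilt for variety.
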(event EventBeginPlay)

(event Collision|EventActorBeginOverlap
  (params (OtherActor :type Actor%20Object%20Reference)))

(event EventTick
  (params (DeltaSeconds :type Float%20%28single-precision%29)))

(fn ConstructionScript
  (bind _bookdisplacevalue_x (Variables|Default|GetBookDisplaceValue_X))
  (bind _bookdisplacevalue_z (Variables|Default|GetBookDisplaceValue_Z))
  (if (Variables|Default|GetRandomize)
    (Math|Random|SetRandomStreamSeed (Variables|Default|GetSeed) (Math|Random|RandomInteger 9999)))
  (for _index (range 0 (- (Variables|Default|GetNumberOfBooks) 1))
    (bind _returnvalue (AddComponent|AddStaticMeshComponent false (Math|Transform|MakeTransform (Variables|Default|GetLocation) "0, 0, 0" "1.000000,1.000000,1.000000")))
    (Components|StaticMesh|SetStaticMesh _returnvalue (Utilities|Array|Get(acopy) (Variables|Default|GetBooks_Data) (Math|Random|RandomIntegerinRangefromStream (Variables|Default|GetSeed) 0 (- (Utilities|Array|Length (Variables|Default|GetBooks_Data)) 1))))
    (Variables|Default|SetLocation (Math|Vector|MakeVector (.x (Variables|Default|GetLocation)) (- (+ (.y (Variables|Default|GetLocation)) (.y (.Min (Components|StaticMesh|GetLocalBounds _returnvalue)))) (Variables|Default|GetDistanceBeetweenBooks)) (.z (Variables|Default|GetLocation))))
    (if (Class|KismetMathLibrary|RandomBoolwithWeightfromStream (Variables|Default|GetSeed) (Variables|Default|GetBalanceBookFliped))
      (Transformation|SetRelativeRotation _returnvalue "0.000000,180.000000,0.000000" false false)
      (Transformation|SetRelativeLocation _returnvalue (Math|Vector|MakeVector (- (.x (.Min (Components|StaticMesh|GetLocalBounds _returnvalue))) (.x (.Max (Components|StaticMesh|GetLocalBounds _returnvalue)))) (+ (.y (Variables|/Script/Engine.SceneComponent|GetRelativeLocation _returnvalue)) (- (.y (.Min (Components|StaticMesh|GetLocalBounds _returnvalue))) (.y (.Max (Components|StaticMesh|GetLocalBounds _returnvalue))))) (.z (Variables|/Script/Engine.SceneComponent|GetRelativeLocation _returnvalue))) false false))
    (if (Math|Random|RandomBoolfromStream (Variables|Default|GetSeed))
      (Transformation|SetRelativeLocation _returnvalue (Math|Vector|MakeVector (+ (.x (Variables|/Script/Engine.SceneComponent|GetRelativeLocation _returnvalue)) (Math|Random|RandomFloatinRangefromStream (Variables|Default|GetSeed) (* _bookdisplacevalue_x -1.0) _bookdisplacevalue_x)) (.y (Variables|/Script/Engine.SceneComponent|GetRelativeLocation _returnvalue)) (.z (Variables|/Script/Engine.SceneComponent|GetRelativeLocation _returnvalue))) false false))
    (if (Math|Random|RandomBoolfromStream (Variables|Default|GetSeed))
      (Transformation|SetRelativeLocation _returnvalue (Math|Vector|MakeVector (.x (Variables|/Script/Engine.SceneComponent|GetRelativeLocation _returnvalue)) (.y (Variables|/Script/Engine.SceneComponent|GetRelativeLocation _returnvalue)) (+ (.z (Variables|/Script/Engine.SceneComponent|GetRelativeLocation _returnvalue)) (Math|Random|RandomFloatinRangefromStream (Variables|Default|GetSeed) (* _bookdisplacevalue_z -1.0) _bookdisplacevalue_z))) false false))
    (if (Math|Random|RandomBoolfromStream (Variables|Default|GetSeed))
      (Transformation|SetRelativeRotation _returnvalue (Math|Rotator|MakeRotator (.roll (Variables|/Script/Engine.SceneComponent|GetRelativeRotation _returnvalue)) (+ (.pitch (Variables|/Script/Engine.SceneComponent|GetRelativeRotation _returnvalue)) (Math|Random|RandomFloatinRangefromStream (Variables|Default|GetSeed) (* (Variables|Default|GetMaxRotation) -1.0) (Variables|Default|GetMaxRotation))) (.yaw (Variables|/Script/Engine.SceneComponent|GetRelativeRotation _returnvalue))) false false))))