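; A modular stone block wall actor that randomizes the look of its nineteen block components.
; The construction script gives each block a weighted chance of visibility from PercentageOfStoneVisible and a random Y scale between MinimumScale and MaximumScale.
; Both draws use the Seed stream, which gets a new random seed on every construction, so the layout changes whenever the script reruns.
; The event graph holds no active logic.
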(event EventBeginPlay)

(event Collision|EventActorBeginOverlap
  (params (OtherActor :type Actor%20Object%20Reference)))

(event EventTick
  (params (DeltaSeconds :type Float%20%28single-precision%29)))

(fn ConstructionScript
  (bind _seed (Variables|Default|GetSeed))
  (bind _output_get (Variables|Default|SetStoneBlocks (Utilities|Array|MakeArray (Variables|Default|GetStoneBlock01) (Variables|Default|GetStoneBlock02) (Variables|Default|GetStoneBlock03) (Variables|Default|GetStoneBlock04) (Variables|Default|GetStoneBlock05) (Variables|Default|GetStoneBlock06) (Variables|Default|GetStoneBlock07) (Variables|Default|GetStoneBlock08) (Variables|Default|GetStoneBlock09) (Variables|Default|GetStoneBlock10) (Variables|Default|GetStoneBlock11) (Variables|Default|GetStoneBlock12) (Variables|Default|GetStoneBlock13) (Variables|Default|GetStoneBlock14) (Variables|Default|GetStoneBlock15) (Variables|Default|GetStoneBlock16) (Variables|Default|GetStoneBlock17) (Variables|Default|GetStoneBlock18) (Variables|Default|GetStoneBlock19))))
  (Math|Random|SetRandomStreamSeed (Variables|Default|GetSeed) (Math|Random|RandomInteger 9999))
  (for _array_element _output_get
    (Rendering|SetVisibility _array_element (Class|KismetMathLibrary|RandomBoolwithWeightfromStream _seed (Variables|Default|GetPercentageOfStoneVisible)) false)
    (Transformation|SetRelativeScale3D _array_element (Math|Vector|MakeVector 1.0 (Math|Random|RandomFloatinRangefromStream _seed (Variables|Default|GetMinimumScale) (Variables|Default|GetMaximumScale)) 1.0))))