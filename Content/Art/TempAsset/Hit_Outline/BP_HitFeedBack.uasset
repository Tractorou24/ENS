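; BP_HitFeedBack is an actor that shows hit-flash and outline feedback on its skeletal mesh when the player pawn overlaps it.
; BeginPlay creates dynamic instances of the mesh's first material and of MM_Outline.
; On overlap, if Hit is set, the Appear timeline drives the HitIntensity parameter.
; If Outline is set, the outline instance becomes the overlay material until the overlap ends.
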(event EventBeginPlay
  (bind _skeletalmesh (Variables|Default|GetSkeletalMesh))
  (bind _returnvalue (Rendering|Material|CreateDynamicMaterialInstance "/Game/Art/Materials/MasterMaterials/Outline/MM_Outline.MM_Outline" "None" "None" :!class /Script/Engine.KismetMaterialLibrary))
  (Variables|Default|SetDynamicOverlayMaterial _returnvalue)
  (bind _returnvalue_2 (Rendering|Material|CreateDynamicMaterialInstance (Rendering|Material|GetMaterial _skeletalmesh 0) "None" "None" :!class /Script/Engine.KismetMaterialLibrary))
  (bind _output_get (Variables|Default|SetDynamicMaterial _returnvalue_2))
  (Rendering|Material|SetMaterial _skeletalmesh 0 _output_get))

(event EventTick
  (params (DeltaSeconds :type Float%20%28single-precision%29)))

(event Collision|EventActorBeginOverlap
  (params (OtherActor :type Actor%20Object%20Reference))
  (if (== OtherActor (Game|Player|GetPlayerPawn 0))
    (Utilities|FlowControl|Sequence
      (:then_0
        (if (Variables|Default|GetHit)
          (bind _newtrack_0 (Timeline|Appear PlayFromStart)
            (:Update
              (Rendering|Material|SetScalarParameterValue (Variables|Default|GetDynamicMaterial) "HitIntensity" _newtrack_0 :!class /Script/Engine.MaterialInstanceDynamic)))))
      (:then_1
        (if (Variables|Default|GetOutline)
          (Rendering|Material|SetOverlayMaterial (Variables|Default|GetSkeletalMesh) (Variables|Default|GetDynamicOverlayMaterial) :!class /Script/Engine.MeshComponent))))))

(event Collision|EventActorEndOverlap
  (params (OtherActor :type Actor%20Object%20Reference))
  (if (== OtherActor (Game|Player|GetPlayerPawn 0))
    (if (Variables|Default|GetOutline)
      (Rendering|Material|SetOverlayMaterial (Variables|Default|GetSkeletalMesh) 0 :!class /Script/Engine.MeshComponent))))

(fn ConstructionScript)