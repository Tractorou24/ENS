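; BP_HitFeedBack is an actor that gives visual hit feedback on its skeletal mesh when the player pawn overlaps it.
; On BeginPlay it creates a dynamic material instance from the mesh's first material slot and assigns it back to that slot.
; Overlap begin and end events for the player pawn switch the material's HitIntensity scalar between a high and a baseline value, with no interpolation.
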(event EventBeginPlay
  (bind _skeletalmesh (Variables|Default|GetSkeletalMesh))
  (bind _returnvalue (Rendering|Material|CreateDynamicMaterialInstance _skeletalmesh 0 (Rendering|Material|GetMaterial _skeletalmesh 0) "None" :!class /Script/Engine.PrimitiveComponent))
  (Variables|Default|SetDynamicMaterial _returnvalue)
  (Rendering|Material|SetMaterial _skeletalmesh 0 _returnvalue))

(event EventTick
  (params (DeltaSeconds :type Float%20%28single-precision%29)))

(event Collision|EventActorBeginOverlap
  (params (OtherActor :type Actor%20Object%20Reference))
  (if (== OtherActor (Game|Player|GetPlayerPawn 0))
    (Rendering|Material|SetScalarParameterValue (Variables|Default|GetDynamicMaterial) "HitIntensity" 1e+02 :!class /Script/Engine.MaterialInstanceDynamic)))

(event Collision|EventActorEndOverlap
  (params (OtherActor :type Actor%20Object%20Reference))
  (if (== OtherActor (Game|Player|GetPlayerPawn 0))
    (Rendering|Material|SetScalarParameterValue (Variables|Default|GetDynamicMaterial) "HitIntensity" 1.0 :!class /Script/Engine.MaterialInstanceDynamic)))

(fn ConstructionScript)