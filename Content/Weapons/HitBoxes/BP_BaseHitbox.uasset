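; BP_BaseHitbox is a base weapon hitbox that damages overlapping enemies once each through the Gameplay Ability System.
; Initialize supplies the Weapon and owning Ability, which Tick asserts before scanning every box collider for overlapping EnsEnemyBase actors.
; Each new enemy is recorded in Hits and receives a damage GameplayEffect from the ability avatar's ASC, with magnitude set by caller from the weapon's first-level base attack damage.
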(event EventBeginPlay
  (Variables|Default|SetColliders (Actor|GetComponentsByClass "/Script/Engine.BoxComponent")))

(event EventTick
  (params (DeltaSeconds :type Float%20%28single-precision%29))
  (Class|EnsBlueprintAssert|BlueprintAssert self (Variables|Default|GetIsInitialized))
  (for _array_element (Variables|Default|GetColliders)
    (for _array_element_2 (Collision|GetOverlappingActors _array_element "/Script/ENS.EnsEnemyBase" :!class /Script/Engine.PrimitiveComponent)
      (bind _asens_enemy_base (Utilities|Casting|CastToEnsEnemyBase _array_element_2)
        (:then
          (if (not (Utilities|Set|Contains (Variables|Default|GetHits) _asens_enemy_base))
            (CallFunction|GiveDamage _asens_enemy_base 1.0 (Utilities|Array|Get(acopy) (Variables|/Script/ENS.EnsSkillBase|GetDamagePerLevel (.BaseAttack (Variables|/Script/ENS.BaseWeapon|GetBaseAttack (Variables|Default|GetWeapon))))))
            (Utilities|Set|Add (Variables|Default|GetHits) _asens_enemy_base)))
        (:CastFailed
          (Class|EnsBlueprintAssert|BlueprintAssert self false))))))

(fn ConstructionScript)

(fn GiveDamage
  (params (Target :type Ens%20Character%20Base%20Object%20Reference) (AttackLevel :type Float%20%28double-precision%29) (Damage :type Float%20%28double-precision%29))
  (bind _ability (Variables|Default|GetAbility))
  (bind _returnvalue (Ability|GetAvatarActorfromActorInfo _ability))
  (bind _returnvalue_2 (Ability|GetAbilitySystemComponent _returnvalue))
  (bind _returnvalue_3 (Ability|GameplayEffect|AssignTagSetbyCallerMagnitude (GameplayEffects|MakeOutgoingSpec _returnvalue_2 "/Game/Characters/Player/Abilities/DevelopperTests/BPGE_Damage.BPGE_Damage_C" AttackLevel (GameplayEffects|MakeEffectContext _returnvalue_2)) "(TagName=\"Ability.Damage\")" Damage))
  (GameplayEffects|ApplyGameplayEffectSpecToSelf (Ability|GetAbilitySystemComponent Target) _returnvalue_3)
  (return))

(fn Initialize
  (params (Weapon :type Base%20Weapon%20Object%20Reference) (Ability :type Gameplay%20Ability%20Object%20Reference))
  (Variables|Default|SetWeapon Weapon)
  (Variables|Default|SetAbility Ability)
  (Variables|Default|SetIsInitialized true))