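; BP_SwordAbilityHitBox is a moving hit box for a sword ability that travels a set distance and then disappears.
; On BeginPlay a timer destroys the actor after Distance divided by Speed.
; Each tick it moves forward along its local X axis without sweeping and draws a debug box matching its Box component.
; The graph itself contains no hit or damage handling.
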(event Custom|Destroy
  (Actor|DestroyActor))

(event EventBeginPlay
  (|CallParentFunction)
  (Utilities|Time|SetTimerbyEvent (delegate Custom|Destroy) (/ (Variables|Components|GetDistance) (Variables|Components|GetSpeed))))

(event EventTick
  (params (DeltaSeconds :type Float%20%28single-precision%29))
  (bind _box (Variables|Default|GetBox))
  (|CallParentFunction DeltaSeconds)
  (Rendering|Debug|DrawDebugBox (Transformation|GetWorldLocation _box) (Components|Box|GetScaledBoxExtent _box) "(R=1.000000,G=0.958712,B=0.778539,A=1.000000)" "0, 0, 0" DeltaSeconds 1.0)
  (Transformation|AddActorLocalOffset (* DeltaSeconds (Math|Vector|MakeVector (Variables|Components|GetSpeed) 0.0 0.0)) false false))

(fn ConstructionScript)