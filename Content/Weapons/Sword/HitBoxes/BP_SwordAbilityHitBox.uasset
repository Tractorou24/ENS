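; BP_SwordAbilityHitBox is a hitbox for a sword ability that travels forward like a projectile.
; Each tick it offsets itself along its local X axis by Speed, without sweeping.
; On BeginPlay a timer set to Distance divided by Speed destroys it, capping its travel range.
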(event Custom|Destroy
  (Actor|DestroyActor))

(event EventBeginPlay
  (|CallParentFunction)
  (Utilities|Time|SetTimerbyEvent (delegate Custom|Destroy) (/ (Variables|Components|GetDistance) (Variables|Components|GetSpeed))))

(event EventTick
  (params (DeltaSeconds :type Float%20%28single-precision%29))
  (|CallParentFunction DeltaSeconds)
  (Transformation|AddActorLocalOffset (* DeltaSeconds (Math|Vector|MakeVector (Variables|Components|GetSpeed) 0.0 0.0)) false false))

(fn ConstructionScript)